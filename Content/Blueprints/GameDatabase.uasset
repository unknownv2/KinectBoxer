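; GameDatabase is a Blueprint that serves as a sound cue library for a two-player, round-based target game.
; Each function plays one fixed 2D sound: the welcome, round-start music, player turn and win announcements, round completion, or a target-hit explosion.
; It stores no state and has no active event logic, so playback happens only when these functions are called.
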(event EventBeginPlay)

(event Collision|EventActorBeginOverlap
  (params (OtherActor :type Actor%20Object%20Reference)))

(event EventTick
  (params (DeltaSeconds :type Float%20%28single-precision%29)))

(fn ConstructionScript)

(fn RoundStartSoundtrack
  (Audio|PlaySound2D "/Game/Blueprints/ImportedAudio/Neon_and_Kickboxing_Fade.Neon_and_Kickboxing_Fade"))

(fn Player1begin
  (Audio|PlaySound2D "/Game/Blueprints/ImportedAudio/player1begin.player1begin"))

(fn Player2begin
  (Audio|PlaySound2D "/Game/Blueprints/ImportedAudio/player2begin.player2begin"))

(fn Player1wins
  (Audio|PlaySound2D "/Game/Blueprints/ImportedAudio/player1Wins.player1Wins"))

(fn RoundComplete
  (Audio|PlaySound2D "/Game/Blueprints/ImportedAudio/round_complete.round_complete"))

(fn WelcomeStart
  (Audio|PlaySound2D "/Game/Blueprints/ImportedAudio/welcome.welcome"))

(fn TargetHit
  (Audio|PlaySound2D "/Game/StarterContent/Audio/Explosion01.Explosion01"))

(fn Player2wins
  (Audio|PlaySound2D "/Game/Blueprints/ImportedAudio/player2Wins.player2Wins"))