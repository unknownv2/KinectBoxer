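; Destructible sphere actor that acts as a score target: any actor overlap destroys it and increments Score on the first GlobalVariableDB actor found in the level.
; BeginPlay creates a dynamic material on the Destructible and sets a red vector, though the parameter name is None.
; Component hits apply point damage to the hit actor.
; The self-damaging actor-hit handler only binds inside itself, and older cast-based score and overlap-damage chains are unconnected.
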(event OnComponentHit(Destructible)
  (params (HitComponent :type Primitive%20Component%20Object%20Reference) (OtherActor :type Actor%20Object%20Reference) (OtherComp :type Primitive%20Component%20Object%20Reference) (NormalImpulse :type Vector :default "0, 0, 0") (Hit :type Hit%20Result%20Structure%20%28by%20ref%29))
  (bind (_bblockinghit _binitialoverlap _time _location _impactpoint _normal _impactnormal _physmat _hitactor) (Collision|BreakHitResult Hit))
  (Development|PrintString "Component Hit event fired")
  (Game|Damage|ApplyPointDamage _hitactor 1e+02 _impactpoint Hit 0 OtherActor "/Script/Engine.DamageType"))

(event OnComponentBeginOverlap(Destructible)
  (params (OverlappedComponent :type Primitive%20Component%20Object%20Reference) (OtherActor :type Actor%20Object%20Reference) (OtherComp :type Primitive%20Component%20Object%20Reference) (OtherBodyIndex :type Integer) (bFromSweep :type Boolean) (SweepResult :type Hit%20Result%20Structure%20%28by%20ref%29)))

(event Custom|OnActorHit_Event_0
  (params (SelfActor :type Actor%20Object%20Reference) (OtherActor :type Actor%20Object%20Reference) (NormalImpulse :type Vector) (Hit :type Hit%20Result%20Structure%20%28by%20ref%29))
  (EventDispatchers|AssignOnActorHit (delegate Custom|OnActorHit_Event_0))
  (Development|PrintString "OnActorHitFired")
  (Game|Damage|ApplyPointDamage SelfActor 1e+02 (.ImpactPoint (Collision|BreakHitResult Hit)) Hit 0 OtherActor))

(event EventBeginPlay
  (bind _destructible (Variables|Default|GetDestructible))
  (bind _returnvalue (Rendering|Material|CreateDynamicMaterialInstance _destructible 0 (Rendering|Material|GetMaterial _destructible 0) :!class /Script/Engine.PrimitiveComponent))
  (Rendering|Material|SetVectorParameterValue _returnvalue "None" (Math|Color|MakeColor 255.0 0.0 0.0) :!class /Script/Engine.MaterialInstanceDynamic))

(event Collision|EventActorBeginOverlap
  (params (OtherActor :type Actor%20Object%20Reference))
  (Actor|DestroyActor)
  (bind _outactors (Actor|GetAllActorsOfClass "/Game/GlobalVariableDB.GlobalVariableDB_C"))
  (Math|Integer|IncrementInt (Variables|/Game/GlobalVariableDB.GlobalVariableDB_C|GetScore (Utilities|Array|Get(acopy) _outactors))))

(event EventTick
  (params (DeltaSeconds :type Float%20%28single-precision%29)))

(fn ConstructionScript)